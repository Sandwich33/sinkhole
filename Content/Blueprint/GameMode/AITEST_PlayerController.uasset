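; AITEST_PlayerController is a player controller for AI testing that turns key presses into event dispatcher calls.
; Tab broadcasts ChangeAITab and prints a "Change AI" debug string.
; Number keys 1 through 5 each broadcast their own location dispatcher, leaving the response to whatever binds to them.
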(event `Key|Tab`
  (params (Key :type "Key Structure" :default "AnyKey"))
  (:`Pressed`
    (`self.ChangeAI(Tab)`)
    (`KismetSystemLibrary.PrintString` "Change AI")))

(event `Key|One`
  (params (Key :type "Key Structure" :default "AnyKey"))
  (:`Pressed`
    (`self.onelocation(1)`)))

(event `Key|Two`
  (params (Key :type "Key Structure" :default "AnyKey"))
  (:`Pressed`
    (`self.twolocation(2)`)))

(event `Key|Three`
  (params (Key :type "Key Structure" :default "AnyKey"))
  (:`Pressed`
    (`self.threelocation(3)`)))

(event `Key|Four`
  (params (Key :type "Key Structure" :default "AnyKey"))
  (:`Pressed`
    (`self.fourlocation(4)`)))

(event `Key|Five`
  (params (Key :type "Key Structure" :default "AnyKey"))
  (:`Pressed`
    (`self.fivelocation(5)`)))

(fn `UserConstructionScript`)