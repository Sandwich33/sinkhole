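; AITEST_HUD is a HUD Blueprint that draws the player's health bar in the bottom-left corner of the screen.
; BeginPlay creates a dynamic material instance from M_hpBar.
; Each DrawHUD casts the player pawn to Player_Person, feeds its Hp/MAXHP ratio into the material's healthPercentage parameter, then draws the material with the T_hpBarFrame texture over it.
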(event `self.ReceiveTick`
  (params (DeltaSeconds :type "Float (single-precision)")))

(event `self.ReceiveBeginPlay`
  (bind _returnvalue (`KismetMaterialLibrary.CreateDynamicMaterialInstance` "/Game/HUD/HpBar/M_hpBar.M_hpBar"))
  (set `self.hpBarInstance` _returnvalue))

(event `self.ReceiveDrawHUD`
  (params (SizeX :type Integer) (SizeY :type Integer))
  (bind _returnvalue (- (`.Y` (`KismetMathLibrary.BreakVector2D` (`WidgetLayoutLibrary.GetViewportSize`))) 80.0))
  (bind _asplayer_person (cast `/Game/Blueprint/Characters/Player/Player_Person` (`GameplayStatics.GetPlayerPawn` 0)))
  (`MaterialInstanceDynamic.SetScalarParameterValue` (`self.hpBarInstance`) "healthPercentage" (/ (`/Game/Blueprint/Characters/Person_Character.hp` _asplayer_person) (`/Game/Blueprint/Characters/Person_Character.MAX_HP` _asplayer_person)))
  (`self.DrawMaterialSimple` (`self.hpBarInstance`) 20.0 _returnvalue 350.0 65.0)
  (`self.DrawTextureSimple` "/Game/HUD/HpBar/T_hpBarFrame.T_hpBarFrame" 20.0 _returnvalue 0.1))

(fn `UserConstructionScript`)